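; BP_MainGameMode is the multiplayer game mode that tracks connected players and supports kicking them.
; Login and logout events add or remove each BP_MainPlayerController in a JoinedPlayers array, then trigger UpdatePlayerList.
; After a short delay, UpdatePlayerList tells BP_MainGameState to refresh its player list.
; KickPlayer treats the player ID as an index into JoinedPlayers and calls OwningClientKickPlayer on that controller.
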(event `self.ReceiveBeginPlay`)

(event `self.K2_PostLogin`
  (params (NewPlayer :type "PlayerController Object Reference"))
  (bind _asbp_main_player_controller (cast `/Game/BPs/BP_MainPlayerController` NewPlayer))
  (`KismetArrayLibrary.Array_Add` (`self.JoinedPlayers`) _asbp_main_player_controller)
  (`self.UpdatePlayerList` :!label _label))

(event `self.K2_OnLogout`
  (params (ExitingController :type "Controller Object Reference"))
  (bind _asbp_main_player_controller (cast `/Game/BPs/BP_MainPlayerController` ExitingController))
  (`KismetArrayLibrary.Array_RemoveItem` (`self.JoinedPlayers`) _asbp_main_player_controller)
  (goto _label))

(event `UpdatePlayerList`
  (`KismetSystemLibrary.Delay` 0.5)
  (bind _asbp_main_game_state (cast `/Game/BPs/BP_MainGameState` (`GameplayStatics.GetGameState`)))
  (`/Game/BPs/BP_MainGameState.UpdatePlayerList` _asbp_main_game_state))

(fn `KickPlayer`
  (params (PlayerID :type Integer))
  (`/Game/BPs/BP_MainPlayerController.OwningClientKickPlayer` (`|GetArrayItem` (`self.JoinedPlayers`) PlayerID)))

(fn `UserConstructionScript`)