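; Game instance that handles network failures and leaving online sessions.
; Network and travel error events print the failure type to screen, then share one path that destroys the session for the first player controller.
; A LeaveSession event opens the VRTestMap level and then destroys the session.
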(event `self.HandleNetworkError`
  (params (FailureType :type "ENetworkFailure Enum" :default "NetDriverAlreadyExists") (bIsServer :type Boolean))
  (`KismetSystemLibrary.PrintString` (`|GetEnumeratorNameAsString` FailureType))
  (`DestroySessionCallbackProxy.DestroySession` (`GameplayStatics.GetPlayerController` 0) :!label _label))

(event `self.HandleTravelError`
  (params (FailureType :type "ETravelFailure Enum" :default "NoLevel"))
  (`KismetSystemLibrary.PrintString` (`|GetEnumeratorNameAsString` FailureType))
  (goto _label))

(event `LeaveSession`
  (`GameplayStatics.OpenLevelBySoftObjectPtr` "/Game/maps/VRTestMap.VRTestMap")
  (`DestroySessionCallbackProxy.DestroySession` (`GameplayStatics.GetPlayerController` 0)))